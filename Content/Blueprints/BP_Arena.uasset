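; Arena boundary actor made of inner and outer rectangles, each built from four side components.
; The construction script scales and positions the sides from Length, Width and Size, enlarging the outer ring by Ratio, then applies a shared Visibility toggle.
; On BeginPlay it binds begin-overlap events on all eight sides, and both the inner and outer handlers destroy any overlapping actor without filtering.
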(event Custom|OnComponentBeginOverlap_Event_0
  (params (OtherActor :type Actor%20Object%20Reference) (OtherComp :type Primitive%20Component%20Object%20Reference) (OtherBodyIndex :type Integer) (bFromSweep :type Boolean) (SweepResult :type Hit%20Result%20Structure%20%28by%20ref%29))
  ;[1 0.177 0] Overlapping OuterArena
  (Actor|DestroyActor OtherActor))

(event Custom|OnComponentBeginOverlap_Event_1
  (params (OtherActor :type Actor%20Object%20Reference) (OtherComp :type Primitive%20Component%20Object%20Reference) (OtherBodyIndex :type Integer) (bFromSweep :type Boolean) (SweepResult :type Hit%20Result%20Structure%20%28by%20ref%29))
  ;[0 1 0.01084] Overlapping InnerArena
  (Actor|DestroyActor OtherActor))

(event EventBeginPlay
  ;[1 0.177 0] Overlapping OuterArena
  (Collision|AssignOnComponentBeginOverlap (Variables|Default|GetOuterLeft) (delegate Custom|OnComponentBeginOverlap_Event_0))
  (Collision|AssignOnComponentBeginOverlap (Variables|Default|GetOuterRight) (delegate Custom|OnComponentBeginOverlap_Event_0))
  (Collision|AssignOnComponentBeginOverlap (Variables|Default|GetOuterUp) (delegate Custom|OnComponentBeginOverlap_Event_0))
  (Collision|AssignOnComponentBeginOverlap (Variables|Default|GetOuterDown) (delegate Custom|OnComponentBeginOverlap_Event_0))
  ;[0 1 0.01084] Overlapping InnerArena
  (Collision|AssignOnComponentBeginOverlap (Variables|Default|GetInnerLeft) (delegate Custom|OnComponentBeginOverlap_Event_1))
  (Collision|AssignOnComponentBeginOverlap (Variables|Default|GetInnerRight) (delegate Custom|OnComponentBeginOverlap_Event_1))
  (Collision|AssignOnComponentBeginOverlap (Variables|Default|GetInnerUp) (delegate Custom|OnComponentBeginOverlap_Event_1))
  (Collision|AssignOnComponentBeginOverlap (Variables|Default|GetInnerDown) (delegate Custom|OnComponentBeginOverlap_Event_1)))

(fn ConstructionScript
  (Utilities|FlowControl|Sequence
    (:then_0
      (|Inner_ScaleSides))
    (:then_1
      (|Inner_TransformSides))
    (:then_2
      (|Outer_ScaleSides))
    (:then_3
      (|Outer_TransformSides))
    (:then_4
      (Rendering|SetVisibility))))