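; Missile projectile Blueprint that explodes when it overlaps an actor tagged "Enemy", ignoring all other actors.
; On impact it deals direct damage plus full, falloff-free radial damage of the same amount, blockable on WorldStatic, so the struck enemy can take both.
; It then spawns an explosion emitter and destroys itself.
; The construction script applies the ParticleTemplate variable as the missile's particle effect.
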(event EventBeginPlay)

(event EventTick
  (params (DeltaSeconds :type Float%20%28single-precision%29)))

(event EventActorBeginOverlap
  (params (OtherActor :type Actor%20Object%20Reference))
  (bind _self self)
  (bind _damage (Variables|Default|GetDamage))
  (bind _returnvalue (Transformation|GetActorLocation _self))
  (if (Actor|ActorHasTag OtherActor "Enemy")
    (Game|Damage|ApplyDamage OtherActor _damage 0 0)
    (Game|Damage|ApplyRadialDamage _damage _returnvalue (Variables|Default|GetRadius) 0 0 0 0 true "ECC_WorldStatic")
    (Effects|SpawnEmitteratLocation "/Game/StarterContent/Particles/P_Explosion.P_Explosion" _returnvalue)
    (Actor|DestroyActor)))

(fn ConstructionScript
  (Effects|Components|ParticleSystem|SetTemplate (Variables|Default|GetParticleTemplate)))