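; BP_Floor is an actor that procedurally builds a strip of floor tiles in its construction script, with no active event logic.
; A loop from Index through Quantity, inclusive, adds static mesh components using FloorMesh and Material.
; Each tile is scaled from Length and Width over 100 with zero Z scale.
; Tiles are spaced by Length along world X at absolute positions, independent of the actor's location.
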(event EventBeginPlay)

(event EventActorBeginOverlap
  (params (OtherActor :type Actor%20Object%20Reference)))

(event EventTick
  (params (DeltaSeconds :type Float%20%28single-precision%29)))

(fn ConstructionScript
  (while (<= (LocalVariables|GetIndex) (Variables|Default|GetQuantity))
    (bind _returnvalue (AddComponent|AddStaticMeshComponent false))
    (Components|StaticMesh|SetStaticMesh _returnvalue (Variables|Default|GetFloorMesh))
    (Transformation|SetWorldScale3D _returnvalue (Math|Vector|MakeVector (/ (Variables|Default|GetLength) 1e+02) (/ (Variables|Default|GetWidth) 1e+02) 0.0))
    (Transformation|SetWorldLocation _returnvalue (Math|Vector|MakeVector (* (LocalVariables|GetIndex) (Variables|Default|GetLength)) 0.0 0.0) false)
    (Rendering|Material|SetMaterial _returnvalue 0 (Variables|Default|GetMaterial))
    (LocalVariables|SetIndex (+ (LocalVariables|GetIndex) 1))))