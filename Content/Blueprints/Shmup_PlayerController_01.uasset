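; Player controller for a shoot 'em up that moves the player's character and toggles the pause menu.
; BeginPlay caches the player pawn as DefaultCharacter_01, and the forward and right axis inputs share one AddMovementInput call on it.
; The PauseMenu action toggles pause, input mode and cursor, creating a PauseScene widget on pause and calling Remove on the found PauseScene list on resume.
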(event EventBeginPlay
  (bind _asdefault_character_01 (Utilities|Casting|CastToDefaultCharacter_01 (Game|GetPlayerCharacter 0))))

(event Input|ActionEvents|InputActionPauseMenu
  ;[1 1 1] Add pause menu
  (:Pressed
    (if (Game|IsGamePaused)
      (Game|SetGamePaused false)
      (Input|SetInputModeGameOnly)
      (Variables|Default|SetbShowMouseCursor false)
      (bind _foundwidgets (Widget|GetAllWidgetsOfClass "/Game/Menu/Scenes/PauseScene.PauseScene_C" true))
      (Utilities|Array|RemoveItem _foundwidgets 0)
      (else
        (Game|SetGamePaused true)
        (Input|SetInputModeUIOnly 0 0 true)
        (Variables|Default|SetbShowMouseCursor true)
        (bind _returnvalue (UserInterface|CreateWidget "/Game/Menu/Scenes/PauseScene.PauseScene_C"))
        (UserInterface|Viewport|AddtoViewport _returnvalue 0)))))

(event Input|AxisEvents|InputAxisMovementForward
  (params (AxisValue :type Float%20%28single-precision%29))
  (Pawn|Input|AddMovementInput (stale EventBeginPlay _asdefault_character_01) (Math|Vector|MakeVector AxisValue (stale Input|AxisEvents|InputAxisMovementRight AxisValue) 0.0) 1.0 false))

(event Input|AxisEvents|InputAxisMovementRight
  (params (AxisValue :type Float%20%28single-precision%29))
  (Pawn|Input|AddMovementInput (stale EventBeginPlay _asdefault_character_01) (Math|Vector|MakeVector (stale Input|AxisEvents|InputAxisMovementForward AxisValue) AxisValue 0.0) 1.0 false))

(fn ConstructionScript)