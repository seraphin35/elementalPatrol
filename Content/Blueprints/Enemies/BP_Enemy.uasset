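; BP_Enemy is an enemy actor that moves forward, hurts the player on contact and awards score when killed.
; Tick offsets it along its forward vector by MovementSpeed without sweeping, and overlapping a BP_PawnCharacter applies one point of damage to it.
; Incoming damage reduces HP; a lethal hit adds floored Points to player 0's score, then destroys the enemy.
; The construction script sets its actor Tags from UTags.
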(event EventActorBeginOverlap
  (params (OtherActor :type Actor%20Object%20Reference))
  (bind _asbp_pawn_character (Utilities|Casting|CastToBP_PawnCharacter OtherActor))
  (Game|Damage|ApplyDamage _asbp_pawn_character 1.0 0 0))

(event EventTick
  (params (DeltaSeconds :type Float%20%28single-precision%29))
  (Transformation|AddActorWorldOffset (* (Math|Vector|GetForwardVector) (* DeltaSeconds (Variables|Default|GetMovementSpeed)))))

(event EventAnyDamage
  (params (Damage :type Float%20%28single-precision%29) (DamageType :type Damage%20Type%20Object%20Reference) (InstigatedBy :type Controller%20Object%20Reference) (DamageCauser :type Actor%20Object%20Reference))
  (if (<= (- (Variables|Default|GetHP) Damage) 0.0)
    (bind _asbp_pawn_character (Utilities|Casting|CastToBP_PawnCharacter (Game|Player|GetPlayerPawn 0)))
    (Default|IncrementScore _asbp_pawn_character (Math|Float|Floor (Variables|Default|GetPoints)))
    (Actor|DestroyActor)
    (else
      (Variables|Default|SetHP (- (Variables|Default|GetHP) Damage)))))

(fn ConstructionScript
  (Variables|Default|SetTags (Variables|Default|GetUTags)))