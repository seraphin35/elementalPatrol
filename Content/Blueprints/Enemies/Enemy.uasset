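; Enemy actor that travels along a spline path and can be destroyed by damage.
; Each tick it advances a fixed distance along the referenced spline blueprint, matching the spline's location and rotation without sweeping, so speed depends on frame rate.
; It destroys itself on reaching the spline's end or when incoming damage depletes its HP.
; The construction script copies UTags into the actor's Tags.
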(event EventBeginPlay)

(event EventAnyDamage
  (params (Damage :type Float%20%28single-precision%29) (DamageType :type Damage%20Type%20Object%20Reference) (InstigatedBy :type Controller%20Object%20Reference) (DamageCauser :type Actor%20Object%20Reference))
  (if (<= (- (Variables|Default|GetHP) Damage) 0.0)
    (Actor|DestroyActor)
    (else
      (Variables|Default|SetHP (- (Variables|Default|GetHP) Damage)))))

(event EventTick
  (params (DeltaSeconds :type Float%20%28single-precision%29))
  (bind _spline_blueprint (Variables|Default|GetSpline_BluePrint))
  (Variables|Default|SetDistance%20Along%20Spline (+ (Variables|Default|GetDistance%20Along%20Spline) 5.0))
  (if (<= (Spline|GetSplineLength _spline_blueprint) (Variables|Default|GetDistance%20Along%20Spline))
    (Actor|DestroyActor)
    (else
      (Transformation|SetActorLocation self (Class|SplineComponent|GetWorldLocationatDistanceAlongSpline _spline_blueprint (Variables|Default|GetDistance%20Along%20Spline)) false)
      (Transformation|SetActorRotation (Class|SplineComponent|GetWorldRotationatDistanceAlongSpline (Variables|/Game/Blueprints/Spline.Spline_C|GetSpline (Variables|Default|GetSpline_BluePrint)) (Variables|Default|GetDistance%20Along%20Spline))))))

(event EventActorBeginOverlap
  (params (OtherActor :type Actor%20Object%20Reference)))

(fn ConstructionScript
  (Variables|Default|SetTags (Variables|Default|GetUTags)))