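; BP_Zone is a sizable zone actor that switches an overlapping player pawn to its weapon while active and loses one health point per overlapping enemy.
; When depleted, it deactivates, reverts the player's weapon if it matches the zone's, and regenerates on a looping timer until full health reactivates it.
; A text render shows health, and the construction script applies size and material.
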(event Custom|Event%20Zone%20Regeneration
  (bind _output_get (Variables|Default|SetHP (+ (Variables|Default|GetHP) 1)))
  (CallFunction|SetTextHealthPoint _output_get)
  (if (>= _output_get (Variables|Default|GetHP_Max))
    (CallFunction|EventZoneActivated)))

(event Custom|Event%20Zone%20Activated
  (Utilities|Time|ClearTimerbyFunctionName self "Event Zone Regeneration")
  (Variables|Default|SetActive true))

(event Custom|Event%20Zone%20Deactivated
  (Variables|Default|SetActive false)
  (Utilities|Time|SetTimerbyFunctionName self "Event Zone Regeneration" (Variables|Default|GetRegenerationRate) true)
  (bind _asbp_pawn_character (Utilities|Casting|CastToBP_PawnCharacter (Game|Player|GetPlayerPawn 0)))
  (if (== (Variables|/Game/Blueprints/BP_PawnCharacter.BP_PawnCharacter_C|GetWeaponType _asbp_pawn_character) (Variables|Default|GetWeaponId))
    (Default|WeaponSwitch _asbp_pawn_character "NewEnumerator0")))

(event EventActorBeginOverlap
  (params (OtherActor :type Actor%20Object%20Reference))
  (if (Variables|Default|GetActive)
    (if (Actor|ActorHasTag OtherActor "Enemy")
      (CallFunction|SetTextHealthPoint (- (Variables|Default|GetHP) 1))
      (if (<= (- (Variables|Default|GetHP) 1) 0)
        (CallFunction|EventZoneDeactivated)
        (else
          (Variables|Default|SetHP (- (Variables|Default|GetHP) 1))))
      (else
        (bind _asbp_pawn_character (Utilities|Casting|CastToBP_PawnCharacter OtherActor))
        (Default|WeaponSwitch _asbp_pawn_character (Variables|Default|GetWeaponId))))))

(event EventBeginPlay
  (bind _output_get (Variables|Default|SetHP (Variables|Default|GetHP_Max)))
  (CallFunction|SetTextHealthPoint _output_get))

(fn ConstructionScript
  (Utilities|FlowControl|Sequence
    (:then_0
      (|SetScale))
    (:then_1
      (Rendering|Material|SetMaterial 0 (Variables|Default|GetMaterial)))))

(fn SetTextHealthPoint
  (params (HP :type Integer :default 0))
  (Rendering|Components|TextRender|SetText (Variables|Default|GetHealthPointsRendering) (Utilities|String|ToString(Integer) HP)))