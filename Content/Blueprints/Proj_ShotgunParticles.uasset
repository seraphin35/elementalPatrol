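; Shotgun particle projectile Blueprint that damages enemies it overlaps.
; On overlap with an actor tagged "Enemy", it applies its Damage value, spawns an explosion emitter at its own location and destroys itself.
; The Construction Script sets the particle template from the ParticleTemplate variable.
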(event EventBeginPlay)

(event EventTick
  (params (DeltaSeconds :type Float%20%28single-precision%29)))

(event EventActorBeginOverlap
  (params (OtherActor :type Actor%20Object%20Reference))
  (if (Actor|ActorHasTag OtherActor "Enemy")
    (Game|Damage|ApplyDamage OtherActor (Variables|Default|GetDamage) 0 0)
    (Effects|SpawnEmitteratLocation "/Game/StarterContent/Particles/P_Explosion.P_Explosion" (Transformation|GetActorLocation self))
    (Actor|DestroyActor)))

(fn ConstructionScript
  (Effects|Components|ParticleSystem|SetTemplate (Variables|Default|GetParticleTemplate)))