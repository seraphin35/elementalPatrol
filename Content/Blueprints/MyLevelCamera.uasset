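; MyLevelCamera is a placeable level camera that becomes the view target of player controller 0 on BeginPlay.
; Its construction script applies exposed variables to the CameraBoon and Camera, setting arm length, world rotation, projection mode, ortho width and aspect ratio.
; A non-zero AspectRatio also turns on aspect ratio constraint, so zero leaves the view unconstrained.
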(event EventBeginPlay
  (Game|Player|SetViewTargetwithBlend (Game|GetPlayerController 0) self 0.0 "VTBlend_Linear" 0.0 false))

(fn ConstructionScript
  (bind _cameraboon (Variables|Default|GetCameraBoon))
  (bind _camera (Variables|Default|GetCamera))
  (Variables|/Script/Engine.SpringArmComponent|SetTargetArmLength _cameraboon (Variables|Default|GetArmLength))
  (Transformation|SetWorldRotation _cameraboon (Variables|Default|GetCameraRotation) false)
  (Variables|/Script/Engine.CameraComponent|SetOrthoWidth _camera (Variables|Default|GetOrthoWidth))
  (Variables|/Script/Engine.CameraComponent|SetProjectionMode _camera (Variables|Default|GetProjectionMode))
  (Variables|/Script/Engine.CameraComponent|SetbConstrainAspectRatio _camera (!= (Variables|Default|GetAspectRatio) 0.0))
  (Variables|/Script/Engine.CameraComponent|SetAspectRatio _camera (Variables|Default|GetAspectRatio)))