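; Player controller for a shmup that toggles the pause menu from the PauseMenu input action.
; Pausing switches to UI-only input, shows the cursor and adds a new PauseScene widget to the viewport.
; Unpausing restores game-only input, hides the cursor and looks up top-level PauseScene widgets for removal.
; The GameOver event is an empty stub.
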(event Custom|GameOver)

(event Input|ActionEvents|InputActionPauseMenu
  ;[1 1 1] Add pause menu
  (:Pressed
    (if (Game|IsGamePaused)
      (Game|SetGamePaused false)
      (Input|SetInputModeGameOnly)
      (Variables|Default|SetbShowMouseCursor false)
      (bind _foundwidgets (Widget|GetAllWidgetsOfClass "/Game/Menu/Scenes/PauseScene.PauseScene_C" true))
      (Utilities|Array|RemoveItem _foundwidgets 0)
      (else
        (Game|SetGamePaused true)
        (Input|SetInputModeUIOnly 0 0 true)
        (Variables|Default|SetbShowMouseCursor true)
        (bind _returnvalue (UserInterface|CreateWidget "/Game/Menu/Scenes/PauseScene.PauseScene_C"))
        (UserInterface|Viewport|AddtoViewport _returnvalue 0)))))

(fn ConstructionScript)