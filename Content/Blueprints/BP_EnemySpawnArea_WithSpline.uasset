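; Enemy spawn area that periodically spawns enemies at points along a line and hands each a spline Blueprint reference.
; The construction script lays evenly spaced arrow components across the width and scales a visual to match.
; When active, BeginPlay gathers Root's children as spawn points and starts a looping timer.
; Spawns occur only within a start/stop window tracked in Tick, using random points for location and facing.
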(event Custom|SpawnEnemy
  (bind _spawnquantity (Variables|Default|GetSpawnQuantity))
  (bind _spawnpoints (Variables|Default|GetSpawnPoints))
  (bind _returnvalue (Math|Random|RandomIntegerinRange 0 _spawnquantity))
  (bind _item (Utilities|Array|Get(acopy) _spawnpoints _returnvalue))
  (if (and (<= (Variables|Default|GetStartTime) (stale EventTick _output_get)) (<= (stale EventTick _output_get) (Variables|Default|GetStopTime)))
    (bind _returnvalue_2 (Game|SpawnActorfromClass (Variables|Default|GetEnemyClass) (Math|Transform|MakeTransform (Transformation|GetWorldLocation _item) (Math|Conversions|RotationFromXVector (Math|Vector|GetForwardVector _item))) false 0))
    (bind _asenemy (Utilities|Casting|CastToEnemy _returnvalue_2))
    (Variables|/Game/Blueprints/Enemies/Enemy.Enemy_C|SetSpline_BluePrint _asenemy (Variables|Default|GetSpline_BluePrint))))

(event EventBeginPlay
  (if (Variables|Default|GetActive)
    (Variables|Default|SetSpawnPoints (Components|GetChildrenComponents (Variables|Default|GetRoot) true))
    (Utilities|Time|SetTimerbyFunctionName self "SpawnEnemy" (Variables|Default|GetTimer) true)))

(event EventTick
  (params (DeltaSeconds :type Float%20%28single-precision%29))
  (bind _output_get (Variables|Default|SetTime%20from%20Beginning (+ DeltaSeconds (Variables|Default|GetTime%20from%20Beginning)))))

(fn ConstructionScript
  (LocalVariables|SetStep (/ (Variables|Default|GetWidth) (Math|Conversions|ToFloat(Integer) (Variables|Default|GetSpawnQuantity))))
  (LocalVariables|SetStart (- 0.0 (/ (Variables|Default|GetWidth) 2.0)))
  (while (<= (LocalVariables|GetIndexLoop) (Variables|Default|GetSpawnQuantity))
    (bind _returnvalue (AddComponent|AddArrowComponent false (Math|Conversions|ToTransform(Vector) (Math|Vector|MakeVector 0.0 (+ (LocalVariables|GetStart) (* (LocalVariables|GetIndexLoop) (LocalVariables|GetStep))) 0.0))))
    (Class|ArrowComponent|SetArrowColorNew _returnvalue "(R=1.000000,G=1.000000,B=1.000000,A=1.000000)")
    (LocalVariables|SetIndexLoop (+ (LocalVariables|GetIndexLoop) 1)))
  (Transformation|SetRelativeScale3D (Variables|Default|GetVisual) (Math|Vector|MakeVector 1.0 (+ (* (LocalVariables|GetStart) -1.0) (LocalVariables|GetStep)) 1.0)))