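; DefaultCharacter_01 is an aircraft character that fires projectiles while Space is held.
; The construction script scales the main mesh and builds four weapon specs, each pairing spawn points with an optional UFO material.
; Tick polls the key behind a 0.3-second cooldown, and Fire spawns Projectiles_01 at each point of the WeaponType spec, passing its material as color.
; A separate ChangeMaterial function reskins the jet body and wings.
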(event EventBeginPlay)

(event EventActorBeginOverlap
  (params (OtherActor :type Actor%20Object%20Reference)))

(event EventTick
  (params (DeltaSeconds :type Float%20%28single-precision%29))
  (if (and (Game|Player|IsInputKeyDown (Game|GetPlayerController 0) "SpaceBar") (Variables|Default|GetWeapon%20Ready))
    (Variables|Default|SetWeapon%20Ready false)
    (CallFunction|Fire)
    (Utilities|FlowControl|Delay 0.3)
    (Variables|Default|SetWeapon%20Ready true)))

(fn ConstructionScript
  (Transformation|SetWorldScale3D (Variables|Default|GetMainMesh) (Math|Conversions|ToVector(Float) (Variables|Default|GetMeshScale)))
  (Variables|Default|SetListWeapon (Utilities|Array|MakeArray (Utilities|Struct|MakeWeaponSpec 0 (Utilities|Array|MakeArray (Variables|Default|GetSpawn01))) (Utilities|Struct|MakeWeaponSpec "/Game/Materials/RedUFO.RedUFO" (Utilities|Array|MakeArray (Variables|Default|GetSpawn01))) (Utilities|Struct|MakeWeaponSpec "/Game/Materials/GreenUFO.GreenUFO" (Utilities|Array|MakeArray (Variables|Default|GetSpawn02) (Variables|Default|GetSpawn03))) (Utilities|Struct|MakeWeaponSpec "/Game/Materials/BlueUFO.BlueUFO" (Utilities|Array|MakeArray (Variables|Default|GetSpawn01) (Variables|Default|GetSpawn02) (Variables|Default|GetSpawn03))))))

(fn Fire
  (bind _listweapon (Variables|Default|GetListWeapon))
  (bind _weapon_type (Variables|Default|GetWeapon%20Type))
  (bind _item (Utilities|Array|Get(acopy) _listweapon _weapon_type))
  (bind (_material _spawnpoints) (Utilities|Struct|BreakWeaponSpec _item))
  (for _array_element _spawnpoints
    (Game|SpawnActorfromClass "/Game/Blueprints/Projectiles_01.Projectiles_01_C" (Transformation|GetWorldTransform _array_element) false _material self)))

(fn ChangeMaterial
  (params (Material :type Material%20Object%20Reference))
  (Rendering|Material|SetMaterial (Variables|Default|GetAircraftBodyJet) 0 Material)
  (Rendering|Material|SetMaterial (Variables|Default|GetAircraftWingsJet) 0 Material))